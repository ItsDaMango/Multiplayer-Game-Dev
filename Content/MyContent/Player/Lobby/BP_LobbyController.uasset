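; BP_LobbyController is the lobby controller that connects player input and incoming chat messages to the chat box widget held in UIRef.
; Client_FillChatBox and Client_AddChat forward a chat history or a single message to UWChatBox.
; The mouse wheel scrolls the chat and Enter focuses it.
; A debug key opens the Lvl_Test level, while BeginPlay, Tick and the construction script are empty.
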(event Custom|Client_AddChat
  (params (Message :type String))
  (Default|ClientAddChat (Variables|/Game/MyContent/Player/Lobby/BP_UI_Lobby.BP_UI_Lobby_C|GetUW_ChatBox (Variables|Default|GetUI_Ref)) Message))

(event Custom|Client_FillChatBox
  (params (Chats :type Array%20of%20Widget%20Object%20References))
  (Default|ClientFillChat (Variables|/Game/MyContent/Player/Lobby/BP_UI_Lobby.BP_UI_Lobby_C|GetUW_ChatBox (Variables|Default|GetUI_Ref)) Chats))

(event EventBeginPlay)

(event EventTick
  (params (DeltaSeconds :type Float%20%28single-precision%29)))

(event Input|KeyboardEvents|DebugKey0
  (params (Key :type Key%20Structure :default "None") (ActionValue :type Input%20Action%20Value%20Structure))
  (:Pressed
    (Game|OpenLevel(byName) "Lvl_Test")))

(event Input|KeyboardEvents|Enter
  (params (Key :type Key%20Structure :default "None"))
  (:Pressed
    (Default|FocusChat (Variables|/Game/MyContent/Player/Lobby/BP_UI_Lobby.BP_UI_Lobby_C|GetUW_ChatBox (Variables|Default|GetUI_Ref)))))

(event Input|MouseEvents|MouseWheelUp
  (params (Key :type Key%20Structure :default "None"))
  (:Pressed
    (Default|Scroll (Variables|/Game/MyContent/Player/Lobby/BP_UI_Lobby.BP_UI_Lobby_C|GetUW_ChatBox (Variables|Default|GetUI_Ref)) true)))

(event Input|MouseEvents|MouseWheelDown
  (params (Key :type Key%20Structure :default "None"))
  (:Pressed
    (Default|Scroll (Variables|/Game/MyContent/Player/Lobby/BP_UI_Lobby.BP_UI_Lobby_C|GetUW_ChatBox (Variables|Default|GetUI_Ref)) false)))

(fn ConstructionScript)