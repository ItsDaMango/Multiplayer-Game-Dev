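; BP_PlayerStart is a player spawn point that can report whether a character is occupying it.
; Its construction script applies a configurable material to two decals.
; CheckSpawnIsEmpty runs a Pawn sphere overlap sized by the DetectionCollision radius and stores the result in DetectedCharacter.
; Despite its name, it returns true when a BP_Character is inside, meaning unsafe, and false when the spawn is clear.
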(event `self.ReceiveTick`
  (params (DeltaSeconds :type "Float (single-precision)")))

(fn `CheckSpawnIsEmpty`
  (returns (failed :type Boolean))
  ;[1 1 1] Check if an actor is in the spawn radius, if not, safe to spawn
  (bind (_outactors _returnvalue) (`KismetSystemLibrary.SphereOverlapActors` (`self.K2_GetActorLocation`) (`SphereComponent.GetScaledSphereRadius` (`self.DetectionCollision`)) (`|MakeArray` "ObjectTypeQuery3" :!type "EObjectTypeQuery Enum") null (`|MakeArray` self :!type "Actor Object Reference")))
  (if _returnvalue
    (for _array_element _outactors
      ;[1 0.312 0.302] If Player is found in the spawn radius, spawn is NOT safe
      (cast `/Game/MyContent/Characters/BP_Character` _array_element
        (:`then`
          (bind _output_get (set `self.bDetectedCharacter` true))
          (return _output_get))
        (:`CastFailed`
          (set `self.bDetectedCharacter` false))))
    (return false)
    (else
      (set `self.bDetectedCharacter` false)
      (return false))))

(fn `UserConstructionScript`
  (`DecalComponent.SetDecalMaterial` (`self.Decal1`) (`self.New Decal Material`))
  (`DecalComponent.SetDecalMaterial` (`self.Decal`) (`self.New Decal Material`)))