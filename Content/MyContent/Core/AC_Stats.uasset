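; AC_Stats is a stats component that stores integer health and max health for its owner.
; SetHealth truncates its input and clamps it between zero and MaxHealth, and DamageHealth and HealHealth both route through it.
; SetMaxHealth truncates and floors the maximum at zero without re-clamping current health.
; IsAlive reports whether health is above zero.
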(fn `DamageHealth`
  (params (Amount :type "Float (double-precision)"))
  (`self.SetHealth` (- (`self.Health`) Amount)))

(fn `HealHealth`
  (params (Amount :type "Float (double-precision)"))
  (`self.SetHealth` (+ (`self.Health`) Amount)))

(fn `IsAlive`
  (returns (ReturnValue :type Boolean))
  (return (> (`self.Health`) 0)))

(fn `SetHealth`
  (params (Health :type "Float (double-precision)"))
  (set `self.Health` (`KismetMathLibrary.Clamp` (`KismetMathLibrary.FTrunc` Health) 0 (`self.MaxHealth`))))

(fn `SetMaxHealth`
  (params (MaxHealth :type "Float (double-precision)"))
  (set `self.MaxHealth` (`KismetMathLibrary.Max` (`KismetMathLibrary.FTrunc` MaxHealth))))