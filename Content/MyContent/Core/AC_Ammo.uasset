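; AC_Ammo is an ammo component that tracks a weapon's clip and its reserve ammo, each with a maximum.
; Functions add, set or consume rounds, and reloading moves only as much reserve as the clip lacks and the reserve holds.
; Every mutator and RepNotify calls the OnAmmoChanged dispatcher, so listeners hear about both local changes and replicated updates.
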(fn `AddAmmo`
  (params (Amount :type Integer))
  (returns (Success :type Boolean))
  (locals (LPreviousAmmo :type Integer))
  (bind _ammo (`self.Ammo`))
  (set `local.LPreviousAmmo` _ammo)
  (set `self.Ammo` (`KismetMathLibrary.Clamp` (+ _ammo Amount) 0 (`self.MaxAmmo`)))
  (`self.OnAmmoChanged`)
  (return (!= (`self.Ammo`) (`local.LPreviousAmmo`))))

(fn `GetAmountToReload`
  (returns (`Reload Amount` :type Integer))
  (bind _output_get (set `self.ReloadAmount` (`KismetMathLibrary.Clamp` (- (`self.MaxWeaponClip`) (`self.WeaponClip`)) 0 (`self.Ammo`))))
  (return _output_get))

(fn `OnRep_Ammo`
  (`self.OnAmmoChanged`))

(fn `OnRep_MaxAmmo`
  (`self.OnAmmoChanged`))

(fn `OnRep_MaxWeaponClip`
  (`self.OnAmmoChanged`))

(fn `OnRep_ReloadAmount`
  (`self.OnAmmoChanged`))

(fn `OnRep_WeaponClip`
  (`self.OnAmmoChanged`))

(fn `ReloadAmmo`
  (locals (LReloadAmount :type Integer))
  (bind _reload_amount (`self.GetAmountToReload`))
  (set `local.LReloadAmount` _reload_amount)
  (set `self.Ammo` (- (`self.Ammo`) (`local.LReloadAmount`)))
  (set `self.WeaponClip` (+ (`self.WeaponClip`) (`local.LReloadAmount`)))
  (`self.OnAmmoChanged`)
  (return))

(fn `SetAmmo`
  (params (Amount :type Integer))
  (set `self.Ammo` (`KismetMathLibrary.Min` Amount (`self.MaxAmmo`)))
  (`self.OnAmmoChanged`))

(fn `SetClip`
  (params (Amount :type Integer))
  (set `self.WeaponClip` (`KismetMathLibrary.Min` Amount (`self.MaxWeaponClip`)))
  (`self.OnAmmoChanged`))

(fn `UseAmmo`
  (`/Engine/EditorBlueprintResources/StandardMacros.DecrementInt` (`self.WeaponClip`)
    (:`  `
      (`self.OnAmmoChanged`)
      (return))))