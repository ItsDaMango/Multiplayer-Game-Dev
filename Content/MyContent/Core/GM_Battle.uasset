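; GM_Battle is the game mode for a multiplayer, kill-based battle played over several rounds, ending in an Ascension round.
; It begins once all expected players join, syncing round and scores from GI_GameInstance to BP_BattleState and BP_PlayerState.
; In Ascension, the player matching the stored key ascends, with a timer retrying until their character exists.
; TryWinGame triggers EndGame, which schedules the next round or returns to lobby; ResetPlayer respawns via a spawn-point sweep.
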(event `Settings`
  (params (RateLimit :type "Float (single-precision)"))
  (`self.SetUserSettings` RateLimit))

(event `SetUserSettings`
  (params (RateLimit :type "Float (single-precision)"))
  (bind _returnvalue (`GameUserSettings.GetGameUserSettings`))
  (`GameUserSettings.SetFrameRateLimit` _returnvalue RateLimit)
  (`GameUserSettings.ApplyNonResolutionSettings` _returnvalue)
  (`KismetSystemLibrary.ExecuteConsoleCommand` "stat FPS" null))

(event `self.ReceiveBeginPlay`)

(event `self.HandleStartingNewPlayer`
  (params (NewPlayer :type "PlayerController Object Reference"))
  ;[1 1 1] On New Player (begin game initially)
  (`parent.HandleStartingNewPlayer` NewPlayer)
  (bind _asgi_game_instance (cast `/Game/MyContent/Core/GI_GameInstance` (`GameplayStatics.GetGameInstance`)))
  (if (and (== (`GameplayStatics.GetNumPlayerStates`) (`/Game/MyContent/Core/GI_GameInstance.PlayerCount` _asgi_game_instance)) (< (`/Game/MyContent/Core/GI_GameInstance.GameRound` _asgi_game_instance) 5))
    (`self.BeginGame`)))

(event `RestartTheGame`
  ;[1 0.1332 0.1929] Restart Game
  (`GameMode.RestartGame`))

(event `Server_EnterLobby`
  ;[1 0.1485 0.2583] Server Travel back to lobby
  (`KismetSystemLibrary.Delay` 0.5)
  (bind _asgi_game_instance (cast `/Game/MyContent/Core/GI_GameInstance` (`GameplayStatics.GetGameInstance`)))
  (`/Game/MyContent/Core/GI_GameInstance.ResetGames` _asgi_game_instance)
  (`MGGameInstance.EndLobbyGame` _asgi_game_instance))

(event `self.K2_PostLogin`
  (params (NewPlayer :type "PlayerController Object Reference"))
  ;[1 1 1] Before Login (OUTDATED USE WHEN NOT USING LOBBY)
  (`self.LoginNoLobby` NewPlayer))

(event `BeginGame`
  ;[0.5882 1 0.6627] Start Game and Add Round
  (if (not (`self.GameStarted`))
    (set `self.GameStarted` true)
    (bind _return (`self.InitialiseGameBegin`))
    ;[1 0.4871 0.0636] If 4th Round, Ascend
    (if _return
      ;[0.5865 1 0.6617] Default Begin Game
      (`KismetSystemLibrary.Delay` 3.0)
      (`self.StartGameDefault`)
      (else
        (`|ExecutionSequence`
          (:`then_0`
            (`KismetSystemLibrary.Delay` 3.0)
            (`self.StartGameDefault`))
          (:`then_1`
            ;[1 0.4871 0.0636] Run Ascend
            (`KismetSystemLibrary.Delay` 1.5)
            (`self.Ascended`)))))))

(event `Ascended`
  ;[0.5608 0.3255 0.07059] Ascend
  ;;[1 0.5427 0.2033] Ascend
  (bind _asgi_game_instance (cast `/Game/MyContent/Core/GI_GameInstance` (`GameplayStatics.GetGameInstance`)))
  (for _array_element (`GameStateBase.PlayerArray` (`GameplayStatics.GetGameState`))
    (bind _asbp_player_state (cast `/Game/MyContent/Player/BP_PlayerState` _array_element))
    (if (== (`/Game/MyContent/Player/BP_PlayerState.CustomName` _asbp_player_state) (`/Game/MyContent/Core/GI_GameInstance.A_PlayerKey` _asgi_game_instance))
      (break)))
  (bind _asbp_character (cast `/Game/MyContent/Characters/BP_Character` (`PlayerState.GetPawn` _asbp_player_state) :!label _label)
    (:`then`
      (bind _output_get (set `self.BP_Char_Ref` _asbp_character))
      (`/Game/MyContent/Characters/BP_Character.TryAscend` _output_get))
    (:`CastFailed`
      (`KismetSystemLibrary.K2_SetTimerDelegate` (delegate `CheckBPValid`) 0.2))))

(event `CheckBPValid`
  ;[0.5608 0.3255 0.07059] Ascend
  (goto _label))

(fn `Ascension Round End`
  (for _array_element (`GameStateBase.PlayerArray` (`GameplayStatics.GetGameState`))
    (bind _asbp_player_state (cast `/Game/MyContent/Player/BP_PlayerState` _array_element))
    (`self.Server_EnterLobby`)
    (set `self.GameStarted` false)))

(fn `EndGame`
  (bind _asbp_battle_state (cast `/Game/MyContent/Core/BP_BattleState` (`GameplayStatics.GetGameState`)))
  (set `self.GameEnded` true)
  (bind _rounds (`/Game/MyContent/Core/BP_BattleState.Rounds` _asbp_battle_state))
  (if (and (< _rounds 4) (not (== _rounds 4)))
    (for _array_element (`GameStateBase.PlayerArray` (`GameplayStatics.GetGameState`))
      (bind _asbp_player_state (cast `/Game/MyContent/Player/BP_PlayerState` _array_element))
      (`/Game/MyContent/Player/BP_PlayerState.OnEndGame` _asbp_player_state))
    (`KismetSystemLibrary.K2_SetTimerDelegate` (`|CreateDelegate` :!event `RestartTheGame`) 3.0)
    (set `self.GameStarted` false)
    (else
      ;[1 0.4811 0.1007] Ascension Round - Restart
      (`self.Ascension Round End`))))

(fn `GetRandomPoint`
  (returns (RandomInt :type Integer))
  (bind _output_get (set `self.RandomInt` (`KismetMathLibrary.RandomIntegerInRange` 0 (`KismetArrayLibrary.Array_LastIndex` (`self.PlayerSpawnPoints`)))))
  (return _output_get))

(fn `InitialiseGameBegin`
  (returns (Return :type Boolean))
  (bind _asgi_game_instance (cast `/Game/MyContent/Core/GI_GameInstance` (`GameplayStatics.GetGameInstance`)))
  (bind _asbp_battle_state (cast `/Game/MyContent/Core/BP_BattleState` (`GameplayStatics.GetGameState`)))
  (bind _result (`/Game/MyContent/Core/GI_GameInstance.GameRoundAdd` _asgi_game_instance))
  (`/Game/MyContent/Core/GI_GameInstance.Server_SetKillsAndScore` _asgi_game_instance)
  (`/Game/MyContent/Core/BP_BattleState.SetRound` _asbp_battle_state _result)
  (return (not (>= _result (`/Game/MyContent/Core/GI_GameInstance.AscensionRound` _asgi_game_instance)))))

(fn `LoginNoLobby`
  (params (`New Player` :type "Controller Object Reference") (PlayWithoutLobby :type Boolean))
  (if PlayWithoutLobby
    (bind _asbp_player_state (cast `/Game/MyContent/Player/BP_PlayerState` (`Controller.PlayerState` `New Player`)))
    (bind _asgi_game_instance (cast `/Game/MyContent/Core/GI_GameInstance` (`GameplayStatics.GetGameInstance`)))
    (`/Game/MyContent/Player/BP_PlayerState.SetCustomName` _asbp_player_state (`KismetStringLibrary.Concat_StrStr` "Player " (`KismetStringLibrary.Conv_IntToString` (`GameplayStatics.GetNumPlayerStates`))))
    (if (== (`GameplayStatics.GetNumPlayerStates`) (`/Game/MyContent/Core/GI_GameInstance.PlayerCount` _asgi_game_instance))
      (`self.BeginGame`))))

(fn `PlayerStateKills`)

(fn `ResetPlayer`
  (params (PlayerController :type "PlayerController Object Reference"))
  (`self.K2_DestroyActor` (`Controller.K2_GetPawn` PlayerController))
  (bind (_failed _playerstart) (`self.SweepSpawnPoints`))
  (`self.RestartPlayerAtPlayerStart` PlayerController _playerstart))

(fn `SetGameModeRound`
  (params (GameModeRound :type Integer)))

(fn `SetKillsToEnd`
  (params (KillsToEnd :type Integer))
  (set `self.TotalKillsToEnd` KillsToEnd))

(fn `StartGameDefault`
  (bind _asgi_game_instance (cast `/Game/MyContent/Core/GI_GameInstance` (`GameplayStatics.GetGameInstance`)))
  (`/Game/MyContent/Core/GI_GameInstance.Server_SetKillsAndScore` _asgi_game_instance)
  (for _array_element (`GameStateBase.PlayerArray` (`GameplayStatics.GetGameState`))
    (bind _asbp_player_state (cast `/Game/MyContent/Player/BP_PlayerState` _array_element))
    (`/Game/MyContent/Player/BP_PlayerState.OnStartGame` _asbp_player_state)))

(fn `SweepSpawnPoints`
  (returns (failed :type Boolean) (PlayerStart :type "/Game/MyContent/Player/BP_PlayerStart Object Reference"))
  (for _array_element (`self.PlayerSpawnPoints`)
    (bind _failed (`/Game/MyContent/Player/BP_PlayerStart.CheckSpawnIsEmpty` _array_element))
    (if (not _failed)
      (return false _array_element)))
  (return true (`KismetArrayLibrary.Array_Random` (`self.PlayerSpawnPoints`))))

(fn `TryWinGame`
  (params (CurrentKills :type Integer))
  (bind _asgi_game_instance (cast `/Game/MyContent/Core/GI_GameInstance` (`GameplayStatics.GetGameInstance`)))
  (bind _asbp_battle_state (cast `/Game/MyContent/Core/BP_BattleState` (`GameplayStatics.GetGameState`)))
  (if (< (`/Game/MyContent/Core/BP_BattleState.Rounds` _asbp_battle_state) (- (`/Game/MyContent/Core/GI_GameInstance.AscensionRound` _asgi_game_instance) 1))
    (if (and (>= (* (`local.CurrentKills`) (`/Game/MyContent/Core/BP_BattleState.Rounds` _asbp_battle_state)) (`self.TotalKillsToEnd`)) (not (`self.GameEnded`)))
      (`self.EndGame`))
    (elif (and (>= (`local.CurrentKills`) (`self.TotalKillsToEnd`)) (not (`self.GameEnded`)) (== (`/Game/MyContent/Core/BP_BattleState.Rounds` _asbp_battle_state) 3))
      (`/Game/MyContent/Core/GI_GameInstance.Server_HighestKills` _asgi_game_instance)
      (`self.EndGame`)
      (elif (not (`/Game/MyContent/Core/AC_Stats.IsAlive` (`/Game/MyContent/Characters/BP_Character.AC_Stats` (`self.BP_Char_Ref`))))
        (`self.EndGame`)))))

(fn `UserConstructionScript`
  (bind _outactors (`GameplayStatics.GetAllActorsOfClass` "/Game/MyContent/Player/BP_PlayerStart.BP_PlayerStart_C"))
  (for _array_element _outactors
    (`KismetArrayLibrary.Array_Add` (`self.PlayerSpawnPoints`) _array_element)))