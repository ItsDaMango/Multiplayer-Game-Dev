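; BP_BattleState holds match state for a multiplayer battle: the round count, an ascended player and player kills.
; Setters update these values; round and ascended-player changes fire notifications, repeated in their OnReps for replication.
; UpdateKillCount binds to each player state's kill-count change event.
; BeginPlay and SetNames are empty, MultiASC only checks validity, and disconnected nodes hold unused naming and ascended-character scaling, material and time-dilation logic.
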(event `self.ReceiveBeginPlay`)

(event `SetNames`)

(event `MultiASC`
  (bind _asgi_game_instance (cast `/Game/MyContent/Core/GI_GameInstance` (`GameplayStatics.GetGameInstance`)))
  (bind _ascendedplayerref (`/Game/MyContent/Core/GI_GameInstance.AscendedPlayerRef` _asgi_game_instance)
    (:`then`)
    (:`else`)))

(fn `AddRound`
  (`self.SetRound` (+ (`self.Rounds`) 1)))

(fn `OnRep_AscendedPlayerRef`
  (`self.OnAscendedPlayerChanged`))

(fn `OnRep_Rounds`
  (`self.OnRoundChanged`))

(fn `SetAscendedPlayer`
  (params (AscendedPlayerRef :type "/Game/MyContent/Player/BP_PlayerState Object Reference"))
  (bind _output_get (set `self.AscendedPlayerRef` AscendedPlayerRef))
  (`self.OnAscendedPlayerChanged`)
  (`KismetSystemLibrary.PrintString` (`KismetSystemLibrary.GetDisplayName` _output_get) true true (struct :`G` 1.0 :`B` 0.471894 :`A` 1.0) 6.0))

(fn `SetKills`
  (params (PlayerKills :type Integer))
  (set `self.PlayerKills` PlayerKills))

(fn `SetRound`
  (params (Rounds :type Integer))
  (set `self.Rounds` Rounds)
  (`self.OnRoundChanged`))

(fn `UpdateKillCount`
  (for _array_element (`GameStateBase.PlayerArray` (`GameplayStatics.GetGameState`))
    (bind _asbp_player_state (cast `/Game/MyContent/Player/BP_PlayerState` _array_element))
    (add `/Game/MyContent/Player/BP_PlayerState.OnKillCountChanged` _asbp_player_state (`|CreateDelegate` :!event `UpdateKillCount`))
    (`KismetSystemLibrary.PrintString` "Hello" true true (struct :`G` 1.0 :`B` 0.56597 :`A` 1.0))))

(fn `UserConstructionScript`)