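; Shotgun weapon Blueprint that overrides damage activation to fire several hitscan pellets per shot, while Fire simply defers to the parent class.
; ActivateDamage traces each pellet in a random direction within a cone that widens by pellet index, so the first stays centered.
; ApplyLineDamage line-traces on Visibility up to Range, ignoring the owning character, and applies point damage on hit, with debug lines drawn for each pellet.
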(fn `ActivateDamage`
  (params (ShootLoc :type "Vector Structure") (ShootDir :type "Vector Structure"))
  (bind _bulletspershot (`self.BulletsPerShot`))
  (for _index (range _bulletspershot)
    (`self.ApplyLineDamage` (`local.ShootLoc`) (`KismetMathLibrary.RandomUnitVectorInConeInDegrees` (`local.ShootDir`) (* _index (/ (`self.SpreadAngle`) _bulletspershot))) "ForDuration"))
  (return))

(fn `ApplyLineDamage`
  (params (`Start Location` :type "Vector Structure") (Direction :type "Vector Structure") (DrawDebugType :type "EDrawDebugTrace Enum" :default "None"))
  (returns (DamageApplied :type "Float (single-precision)"))
  (bind (_outhit _returnvalue) (`KismetSystemLibrary.LineTraceSingle` `Start Location` (+ `Start Location` (* Direction (`self.Range`))) "TraceTypeQuery1" false (`|MakeArray` (`self.CharcterOwner`) :!type "Actor Object Reference") DrawDebugType))
  (if _returnvalue
    (bind _returnvalue_2 (`GameplayStatics.ApplyPointDamage` (`.HitActor` (`GameplayStatics.BreakHitResult` _outhit)) (`self.Damage`) (`local.Direction`) _outhit null self))
    (return _returnvalue_2)))

(fn `Fire`
  (params (ShootLoc :type "Vector Structure") (ShootDir :type "Vector Structure"))
  (returns (Duration :type "Float (single-precision)"))
  (bind _duration (`parent.Fire` ShootLoc ShootDir))
  (return _duration))

(fn `UserConstructionScript`
  (`parent.UserConstructionScript`))