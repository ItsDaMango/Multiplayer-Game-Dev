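; Ammo pickup that adds ammo to the character's held weapon through its AmmoComponent.
; Overrides the pickup, deactivate and reactivate hooks of its parent.
; A looping timeline pulses the decal's scale while active.
; On deactivation it destroys itself if it has no reactivate time, otherwise it stops the pulse and hides the mesh until reactivated.
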(event `self.ReceiveBeginPlay`
  (`parent.ReceiveBeginPlay`)
  (`self.DecalMovement`))

(event `self.ReceiveTick`
  (params (DeltaSeconds :type "Float (single-precision)"))
  (`parent.ReceiveTick` DeltaSeconds))

(event `DecalMovement`
  (bind (_direction _alpha) (`Timeline|TL_Decal` :!via `PlayFromStart` :!label _label)
    (:`Update`
      (`SceneComponent.K2_SetRelativeTransform` (`self.DecalTransform`) (`KismetMathLibrary.MakeTransform` (0.0 0.0 0.0) (struct) (`KismetMathLibrary.Conv_DoubleToVector` (`KismetMathLibrary.Lerp` 0.5 1.0 _alpha))) false false))
    (:`Finished`
      (`self.DecalMovement`))))

(event `StopDecal`
  (goto _label :!via `Stop`))

(fn `OnDeactivate`
  (`parent.OnDeactivate`)
  (if (== (`self.ReactivateTime`) 0.0)
    (`self.K2_DestroyActor`)
    (else
      (`self.StopDecal`)
      (`SceneComponent.SetVisibility` (`self.AmmoPickup`) false false))))

(fn `OnReactive`
  (`parent.OnReactive`)
  (`SceneComponent.SetVisibility` (`self.AmmoPickup`) true false)
  (`self.DecalMovement`))

(fn `Pickup`
  (params (Character :type "/Game/MyContent/Characters/BP_Character Object Reference"))
  (bind _character (`local.Character`)
    (:`then`
      (bind _asbp_weapon (cast `/Game/MyContent/Weapons/BP_Weapon` (`ChildActorComponent.ChildActor` (`/Game/MyContent/Characters/BP_Character.WeaponActor` _character))))
      (`/Game/MyContent/Core/AC_Ammo.AddAmmo` (`/Game/MyContent/Weapons/BP_Weapon.AmmoComponent` _asbp_weapon) (`self.Ammo`)))
    (:`else`)))

(fn `UserConstructionScript`
  (`parent.UserConstructionScript`))