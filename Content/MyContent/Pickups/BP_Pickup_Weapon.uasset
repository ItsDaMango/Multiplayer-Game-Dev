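; Weapon pickup Blueprint, configured by a WeaponAsset, that gives a character a weapon.
; The construction script previews the asset's skeletal mesh.
; Pickup is skipped while the character is reloading; otherwise, with a valid asset, it activates the weapon class, refreshes the client UI and enables shooting.
; Parent deactivate and reactivate hooks are extended to hide and show the mesh.
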(fn `OnDeactivate`
  (`parent.OnDeactivate`)
  (`SceneComponent.SetVisibility` (`self.SkeletalMesh`) false false))

(fn `OnReactive`
  (`parent.OnReactive`)
  (`SceneComponent.SetVisibility` (`self.SkeletalMesh`) true false))

(fn `Pickup`
  (params (Character :type "/Game/MyContent/Characters/BP_Character Object Reference"))
  (if (not (`/Game/MyContent/Characters/BP_Character.IsReloading` Character))
    (bind _weaponasset (`self.WeaponAsset`)
      (:`then`
        (`/Game/MyContent/Characters/BP_Character.ActivateWeapon` Character (`/Game/MyContent/Pickups/BP_DA_WeaponPickup.WeaponClass` _weaponasset))
        (`/Game/MyContent/Characters/BP_Character.Client_UpdateUI` Character)
        (set `/Game/MyContent/Characters/BP_Character.CanShoot` true Character))
      (:`else`))))

(fn `UserConstructionScript`
  (`parent.UserConstructionScript`)
  (bind _weaponasset (`self.WeaponAsset`)
    (:`then`
      (`SkeletalMeshComponent.SetSkeletalMeshAsset` (`self.SkeletalMesh`) (`/Game/MyContent/Pickups/BP_DA_WeaponPickup.SkeletalMesh` _weaponasset)))
    (:`else`)))